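; M-I-M-A is an AI repair character that fixes broken ship systems such as the bridge, engines, oxygen and steering.
; Tick scans an array of the GameMode's broken flags, then pauses itself and sends the pawn to that system's location after a delay.
; On arrival it waits, clears the flag, restarts that system's timer and calls AddStable on the GameMode.
; It then returns to its spawn point, refreshes the array and resumes scanning.
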(event `Repair`
  (switch `int` (`self.Array Index`)
    (:`0`
      (`self.Repair Bridge`))
    (:`1`
      (`self.Repair Doss`))
    (:`2`
      (`self.Repair Engine 1`))
    (:`3`
      (`self.Repair Engine 2`))
    (:`4`
      (`self.Repair Fuel Storage`))
    (:`5`
      (`self.Repair O2H20 Storage`))
    (:`6`
      (`self.Repair O2`))
    (:`7`
      (`self.Repair Staff Maintenance`))
    (:`8`
      (`self.Repair Steering`)))
  (`ExperimentalGameMode.AddStable` (`self.GM`)))

(event `Set Move Location`
  (set `self.MoveLocation` (`|GetArrayItem` (`self.Locations`) (`self.Array Index`)))
  (`self.Move`))

(event `self.ReceiveBeginPlay`
  (set `self.SpawnLocation` (`self.K2_GetActorLocation`))
  (bind _asexperimental_game_mode (cast `ExperimentalGameMode` (`GameplayStatics.GetGameMode`)))
  (set `self.GM` _asexperimental_game_mode)
  (`self.Update Array`))

(event `Move`
  (`KismetSystemLibrary.Delay` 30.0)
  (`|AIMoveTo` self (`self.MoveLocation`) null 30.0
    (:`OnSuccess`
      (`KismetSystemLibrary.Delay` 10.0)
      (`self.Repair`)
      (`|AIMoveTo` self (`self.SpawnLocation`) null 30.0
        (:`OnSuccess`
          (`self.Update Array`)
          (`self.SetActorTickEnabled` true))))))

(event `self.ReceiveTick`
  (params (DeltaSeconds :type "Float (single-precision)"))
  (for (_array_element _array_index) (`self.BrokenArray`)
    (if _array_element
      (set `self.Array Index` _array_index)
      (`self.SetActorTickEnabled` false)
      (`self.Set Move Location`)))
  (`self.Update Array`))

(event `Update Array`
  (bind _gm (`self.GM`))
  (set `self.BrokenArray` (`|MakeArray` (`ExperimentalGameMode.bBridgeBroken` _gm) (`ExperimentalGameMode.bDOSSBroken` _gm) (`ExperimentalGameMode.bEngineBroken_0` _gm) (`ExperimentalGameMode.bEngineBroken_1` _gm) (`ExperimentalGameMode.bFuelStorageBroken` _gm) (`ExperimentalGameMode.bO2H2OStorageBroken` _gm) (`ExperimentalGameMode.bO2RefreshBroken` _gm) (`ExperimentalGameMode.bStaffMainBroken` _gm) (`ExperimentalGameMode.bSteeringBroken` _gm))))

(fn `Repair Bridge`
  (bind _gm (`self.GM`))
  (set `ExperimentalGameMode.bBridgeBroken` false _gm)
  (`ExperimentalGameMode.BridgeTimer` _gm))

(fn `Repair Doss`
  (bind _gm (`self.GM`))
  (set `ExperimentalGameMode.bDOSSBroken` false _gm)
  (`ExperimentalGameMode.DOSSTimer` _gm))

(fn `Repair Engine 1`
  (bind _gm (`self.GM`))
  (set `ExperimentalGameMode.bEngineBroken_0` false _gm)
  (`ExperimentalGameMode.EngineTimer_0` _gm))

(fn `Repair Engine 2`
  (bind _gm (`self.GM`))
  (set `ExperimentalGameMode.bEngineBroken_1` false _gm)
  (`ExperimentalGameMode.EngineTimer_1` _gm))

(fn `Repair Fuel Storage`
  (bind _gm (`self.GM`))
  (set `ExperimentalGameMode.bFuelStorageBroken` false _gm)
  (`ExperimentalGameMode.FuelStorageTimer` _gm))

(fn `Repair O2`
  (bind _gm (`self.GM`))
  (set `ExperimentalGameMode.bO2RefreshBroken` false _gm)
  (`ExperimentalGameMode.O2RefreshTimer` _gm))

(fn `Repair O2H20 Storage`
  (bind _gm (`self.GM`))
  (set `ExperimentalGameMode.bO2H2OStorageBroken` false _gm)
  (`ExperimentalGameMode.O2H2OStorageTimer` _gm))

(fn `Repair Staff Maintenance`
  (bind _gm (`self.GM`))
  (set `ExperimentalGameMode.bStaffMainBroken` false _gm)
  (`ExperimentalGameMode.StaffMainTimer` _gm))

(fn `Repair Steering`
  (bind _gm (`self.GM`))
  (set `ExperimentalGameMode.bSteeringBroken` false _gm)
  (`ExperimentalGameMode.SteeringTimer` _gm))

(fn `UserConstructionScript`)