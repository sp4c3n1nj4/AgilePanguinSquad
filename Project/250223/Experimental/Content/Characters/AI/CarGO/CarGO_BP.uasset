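; CarGO_BP is an AI cargo carrier that shuttles between two patrol points in the experimental game mode.
; On BeginPlay it caches the game mode and starts a Patrol event that drives AI Move To through a PatrolPoints array.
; It pauses briefly after the first point and longer after wrapping back to index zero.
; After that longer pause it resumes only if the game mode's CarGOChargeBroken flag is not set.
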(event `self.ReceiveBeginPlay`
  (bind _asexperimental_game_mode (cast `ExperimentalGameMode` (`GameplayStatics.GetGameMode`)))
  (set `self.GM_REF` _asexperimental_game_mode)
  (`self.Patrol`))

(event `Patrol`
  (`|AIMoveTo` self (`|GetArrayItem` (`self.PatrolPoints`) (`self.PatrolInt`)) null
    (:`OnSuccess`
      (bind _result (`/Engine/EditorBlueprintResources/StandardMacros.IncrementInt` (`self.PatrolInt`))
        (:`  `
          (bind _output_get (set `self.PatrolInt` _result))
          (if (> _output_get 1)
            (set `self.PatrolInt` 0)
            (`KismetSystemLibrary.Delay` 15.0)
            (if (not (`ExperimentalGameMode.bCarGOChargeBroken` (`self.GM_REF`)))
              (`self.Patrol` :!label _label))
            (else
              (`KismetSystemLibrary.Delay` 5.0)
              (goto _label))))))))

(fn `UserConstructionScript`)