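; C2-M2 is an AI pawn Blueprint that wanders between random reachable points and periodically returns to where it spawned.
; A looping Move event waits, then uses AIMoveTo toward a point around its current location, retrying on failure.
; After a random number of successful moves it heads back to spawn, pauses and rerolls the count.
; The move counter is never reset, and a failed return trip has no handler.
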(event `self.ReceiveBeginPlay`
  (set `self.spawnLocation` (`self.K2_GetActorLocation`))
  (`self.SetMoveAmount`)
  (`self.Move`))

(event `Move`
  (`KismetSystemLibrary.Delay` 5.0)
  (`|AIMoveTo` self (`NavigationSystemV1.K2_GetRandomReachablePointInRadius` (`self.K2_GetActorLocation`) 10000.0 null null) null 1000.0
    (:`OnSuccess`
      (bind _result (`/Engine/EditorBlueprintResources/StandardMacros.IncrementInt` (`self.moveInt`))
        (:`  `
          (bind _output_get (set `self.moveInt` _result))
          (if (== _output_get (`self.moveAmount`))
            (`KismetSystemLibrary.Delay` 5.0)
            (`|AIMoveTo` self (`self.spawnLocation`) null
              (:`OnSuccess`
                (`KismetSystemLibrary.Delay` 15.0)
                (`self.SetMoveAmount`)
                (`self.Move`)))
            (else
              (`self.Move`))))))
    (:`OnFail`
      (`self.Move`))))

(event `SetMoveAmount`
  (set `self.moveAmount` (`KismetMathLibrary.RandomIntegerInRange` 3 5)))

(fn `UserConstructionScript`)