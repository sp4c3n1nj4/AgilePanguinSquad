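; S-O-S AI pawn that chases the player once their suspicion hits 100, then returns to its charging port.
; Tick fires the chase through a DoOnce and disables itself, or just disables itself if the game mode flags the SOS charge broken.
; The chase starts a recursive six-second loop lowering suspicion until zero.
; Successfully reaching the port re-enables tick and resets the DoOnce.
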(event `self.ReceiveBeginPlay`
  (bind _asexperimental_character (cast `ExperimentalCharacter` (`GameplayStatics.GetPlayerCharacter` 0)))
  (set `self.Char_REF` _asexperimental_character)
  (bind _asexperimental_game_mode (cast `ExperimentalGameMode` (`GameplayStatics.GetGameMode`)))
  (set `self.GM_REF` _asexperimental_game_mode))

(event `self.ReceiveTick`
  (params (DeltaSeconds :type "Float (single-precision)"))
  (if (== (`ExperimentalCharacter.suspicionPercentage` (`self.Char_REF`)) 100.0)
    (if (not (`ExperimentalGameMode.bSOSChargeBroken` (`self.GM_REF`)))
      (`/Engine/EditorBlueprintResources/StandardMacros.DoOnce` false :!label _label
        (:`Completed`
          (`self.Chase`))))
    (`self.SetActorTickEnabled` false)))

(event `Return`
  (`|AIMoveTo` self (`self.ChargingPortLOC`) null
    (:`OnSuccess`
      (`self.SetActorTickEnabled` true)
      (goto _label :!via `Reset`))))

(event `SusDelay`
  (bind _char_ref (`self.Char_REF`))
  (`KismetSystemLibrary.Delay` 6.0 :!label _label_2)
  (`ExperimentalCharacter.DecreaseSus` _char_ref)
  (if (== (`ExperimentalCharacter.suspicionPercentage` _char_ref) 0.0)
    (`self.Return`)
    (else
      (`self.SusDelay`))))

(event `Chase`
  (`|AIMoveTo` self (0.0 0.0 0.0) (`self.Char_REF`)
    (:`then`
      (goto _label_2))))

(fn `UserConstructionScript`)