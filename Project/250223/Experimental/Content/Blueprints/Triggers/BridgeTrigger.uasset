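; Trigger volume that shows the bridge terminal UI while an ExperimentalCharacter stands inside its box.
; Entering sets the character's BridgeOverlap flag, creates the BridgeTerminal widget on first use, adds it to the viewport and removes the BridgeRoom widget if visible.
; Leaving clears the flag and removes the terminal, keeping its reference for reuse.
; BridgeRoomREF is only checked and removed here, never created.
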(event `self.Box.OnComponentBeginOverlap`
  (params (OverlappedComponent :type "PrimitiveComponent Object Reference") (OtherActor :type "Actor Object Reference") (OtherComp :type "PrimitiveComponent Object Reference") (OtherBodyIndex :type Integer) (bFromSweep :type Boolean) (SweepResult :type "HitResult Structure (by ref)"))
  (bind _bridgeroom_ref (`self.BridgeRoom_REF`))
  (bind _asexperimental_character (cast `ExperimentalCharacter` OtherActor))
  (set `ExperimentalCharacter.bBridgeOverlap` true _asexperimental_character)
  (`/Engine/EditorBlueprintResources/StandardMacros.IsValid` (`self.BridgeTerminal_REF`)
    (:`Is Valid`
      _)
    (:`Is Not Valid`
      (bind _returnvalue (`|CreateWidget` "/Game/Blueprints/HUDs/TriggerText/BridgeTerminal.BridgeTerminal_C"))
      (bind _output_get (set `self.BridgeTerminal_REF` _returnvalue))))
  (`UserWidget.AddToViewport` _output_get 0)
  (`/Engine/EditorBlueprintResources/StandardMacros.IsValid` _bridgeroom_ref
    (:`Is Valid`
      (if (`Widget.IsVisible` _bridgeroom_ref)
        (`Widget.RemoveFromParent` _bridgeroom_ref)))))

(event `self.Box.OnComponentEndOverlap`
  (params (OverlappedComponent :type "PrimitiveComponent Object Reference") (OtherActor :type "Actor Object Reference") (OtherComp :type "PrimitiveComponent Object Reference") (OtherBodyIndex :type Integer))
  (bind _bridgeterminal_ref (`self.BridgeTerminal_REF`))
  (bind _asexperimental_character (cast `ExperimentalCharacter` OtherActor))
  (set `ExperimentalCharacter.bBridgeOverlap` false _asexperimental_character)
  (`/Engine/EditorBlueprintResources/StandardMacros.IsValid` _bridgeterminal_ref
    (:`Is Valid`
      (if (`Widget.IsVisible` _bridgeterminal_ref)
        (`Widget.RemoveFromParent` _bridgeterminal_ref)))))

(fn `UserConstructionScript`)