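; MIMA charging port actor that flags when the player character is within range and blows up when broken.
; Box collision overlaps set MIMAChargeOverlap on ExperimentalCharacter, with debug prints.
; Tick polls APSRDChargeBroken (not a MIMA-named flag) on the ExperimentalGameMode cached at BeginPlay.
; Once that flag is true, it disables its tick, activates the Explosion component and plays a 2D sound.
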(event `self.BoxCollision.OnComponentBeginOverlap`
  (params (OverlappedComponent :type "PrimitiveComponent Object Reference") (OtherActor :type "Actor Object Reference") (OtherComp :type "PrimitiveComponent Object Reference") (OtherBodyIndex :type Integer) (bFromSweep :type Boolean) (SweepResult :type "HitResult Structure (by ref)"))
  (bind _asexperimental_character (cast `ExperimentalCharacter` OtherActor))
  (set `ExperimentalCharacter.bMIMAChargeOverlap` true _asexperimental_character)
  (`KismetSystemLibrary.PrintString` "MIMACharge Overlap = true"))

(event `self.BoxCollision.OnComponentEndOverlap`
  (params (OverlappedComponent :type "PrimitiveComponent Object Reference") (OtherActor :type "Actor Object Reference") (OtherComp :type "PrimitiveComponent Object Reference") (OtherBodyIndex :type Integer))
  (bind _asexperimental_character (cast `ExperimentalCharacter` OtherActor))
  (set `ExperimentalCharacter.bMIMAChargeOverlap` false _asexperimental_character)
  (`KismetSystemLibrary.PrintString` "MIMACharge Overlap = false"))

(event `self.ReceiveTick`
  (params (DeltaSeconds :type "Float (single-precision)"))
  (if (`ExperimentalGameMode.bAPSRDChargeBroken` (`self.GM_REF`))
    (`/Engine/EditorBlueprintResources/StandardMacros.DoOnce` false
      (:`Completed`
        (`self.SetActorTickEnabled` false)
        (`ActorComponent.Activate` (`self.Explosion`) false)
        ;[1 1 1] Daniel, Explosion Here
        (`GameplayStatics.PlaySound2D` null 1.0 1.0 0.0 null null)))))

(event `self.ReceiveBeginPlay`
  (bind _asexperimental_game_mode (cast `ExperimentalGameMode` (`GameplayStatics.GetGameMode`)))
  (set `self.GM_REF` _asexperimental_game_mode))

(fn `UserConstructionScript`)